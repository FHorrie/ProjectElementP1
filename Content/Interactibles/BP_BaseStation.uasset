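; BP_BaseStation is an interactible station that opens and closes the upgrade menu.
; On BeginPlay it caches the first player controller's BP_NewHUD, and its PickUpObject event calls ToggleUpgradeMenu on that HUD.
; The construction script and end-overlap event only call the parent, and the begin-overlap event is disabled.
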(event Collision|EventActorBeginOverlap
  (params (OtherActor :type Actor%20Object%20Reference))
  (|CallParentFunction OtherActor) ; This node is disabled and will not be called.\nDrag off pins to build functionality.
)

(event Collision|EventActorEndOverlap
  (params (OtherActor :type Actor%20Object%20Reference))
  (|CallParentFunction OtherActor))

(event EventPickUpObject
  (params (InteractCharacter :type Shiflix%20Character%20Object%20Reference))
  (Default|ToggleUpgradeMenu (Variables|Default|GetHUD%20Ref)))

(event EventBeginPlay
  (bind _asbp_new_hud (Utilities|Casting|CastToBP_NewHUD (HUD|GetHUD (Game|GetPlayerController 0))))
  (Variables|Default|SetHUD%20Ref _asbp_new_hud))

(fn ConstructionScript
  (|CallParentFunction))