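; BP_Plaza is a level piece for a plaza with three optional walls: end, left and right.
; SetWalls reads a boolean for each wall and passes it to SetWallVisibility, which toggles visibility, children included, and switches collision between query-and-physics and none.
; It runs from both the Construction Script and BeginPlay, so the layout applies when the actor is constructed and again when play starts.
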(event EventBeginPlay
  (CallFunction|SetWalls))

(event Collision|EventActorBeginOverlap
  (params (OtherActor :type Actor%20Object%20Reference)))

(event EventTick
  (params (DeltaSeconds :type Float%20%28single-precision%29)))

(fn ConstructionScript
  (CallFunction|SetWalls))

(fn SetWallVisibility
  (params (isVisible :type Boolean) (wall :type Static%20Mesh%20Component%20Object%20Reference))
  (Rendering|SetVisibility wall isVisible true)
  (if isVisible
    (Collision|SetCollisionEnabled wall "QueryAndPhysics")
    (else
      (Collision|SetCollisionEnabled wall "NoCollision"))))

(fn SetWalls
  (CallFunction|SetWallVisibility (Variables|Default|GetUseEndWall) (Variables|Default|GetWall))
  (CallFunction|SetWallVisibility (Variables|Default|GetUseRightWall) (Variables|Default|GetWall2))
  (CallFunction|SetWallVisibility (Variables|Default|GetUseLeftWall) (Variables|Default|GetWall1)))