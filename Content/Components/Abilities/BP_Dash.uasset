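; BP_Dash is a dash ability that launches its owning Character when used.
; Use multiplies a direction by DashStrength and passes it to LaunchCharacter, overriding existing XY and Z velocity.
; The direction follows horizontal velocity, or actor forward when the character has virtually none.
; FlattenDirection sets a small fixed Z before normalizing, so upward lift is noticeable from standstill but shrinks as speed rises.
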(event EventBeginPlay)

(event EventTick
  (params (DeltaSeconds :type Float%20%28single-precision%29)))

(event EventUse
  (bind _ascharacter (Utilities|Casting|CastToCharacter (Components|GetOwner)))
  (bind _direction (CallFunction|GetDashDirection _ascharacter))
  (Character|LaunchCharacter _ascharacter (* _direction (Variables|Default|GetDashStrength)) true true))

(fn GetDashDirection
  (params (characterPtr :type Character%20Object%20Reference))
  (bind _returnvalue (Transformation|GetVelocity characterPtr))
  (if (< (Math|Vector|VectorLengthXY _returnvalue) 1e-06)
    (return (CallFunction|FlattenDirection (Transformation|GetActorForwardVector characterPtr)))
    (else
      (return (CallFunction|FlattenDirection _returnvalue)))))

(fn FlattenDirection
  (params (direction :type Vector))
  (return (Math|Vector|Normalize (Math|Vector|MakeVector (.x direction) (.y direction) 0.1))))