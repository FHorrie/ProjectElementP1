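; Ability component that gives a ShiflixCharacter a melee attack through an arm actor spawned on BeginPlay and attached in front of it.
; Use and Stop toggle an attacking flag, and Tick calls the arm's Attack while it is set.
; Hitbox overlaps deal point damage scaled by the arm's multiplier, skipping actors with the same instigator.
; Each actor is hit once until the arm stops attacking, which clears the hit list.
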(event Custom|Overlap
  (params (OverlappedComponent :type Primitive%20Component%20Object%20Reference) (OtherActor :type Actor%20Object%20Reference) (OtherComp :type Primitive%20Component%20Object%20Reference) (OtherBodyIndex :type Integer) (bFromSweep :type Boolean) (SweepResult :type Hit%20Result%20Structure%20%28by%20ref%29))
  (bind _shouldhit (CallFunction|ShouldHit OtherActor))
  (if _shouldhit
    (CallFunction|ApplyDamage (Variables|Default|GetDamage) OtherActor OtherComp)))

(event EventBeginPlay
  (bind _returnvalue (CallFunction|SpawnClaw))
  (Variables|Default|Setattack _returnvalue))

(event EventTick
  (params (DeltaSeconds :type Float%20%28single-precision%29))
  (Utilities|FlowControl|Sequence
    (:then_0
      (if (Variables|Default|GetisAttacking)
        (Default|Attack (Variables|Default|Getattack))))
    (:then_1
      (if (not (Variables|/Game/Damage/BP_AttackArm.BP_AttackArm_C|GetisAttacking (Variables|Default|Getattack)))
        (Utilities|Array|Clear (Variables|Default|GetattackedActors))))))

(event EventUse
  (Variables|Default|SetisAttacking true))

(event EventStop
  (Variables|Default|SetisAttacking false))

(event EventEndPlay
  (params (EndPlayReason :type EEndPlayReason%20Enum :default "Destroyed"))
  (Actor|DestroyActor (Variables|Default|Getattack)))

(fn GetHitboxSpawn
  (params (offset :type Float%20%28double-precision%29))
  (bind _returnvalue (Components|GetOwner))
  (bind _returnvalue_2 (Transformation|GetActorForwardVector _returnvalue))
  (return (Math|Transform|MakeTransform (+ (Transformation|GetActorLocation _returnvalue) (* _returnvalue_2 offset)) (Math|Conversions|RotationFromXVector _returnvalue_2) "1.000000,1.000000,1.000000")))

(fn ApplyDamage
  (params (damage :type Float%20%28double-precision%29) (otherActor :type Actor%20Object%20Reference) (component :type Primitive%20Component%20Object%20Reference))
  (bind _aspawn (Utilities|Casting|CastToPawn (Components|GetOwner)))
  (if (!= (Variables|/Script/Engine.Actor|GetInstigator _aspawn) (Variables|/Script/Engine.Actor|GetInstigator otherActor))
    (Game|Damage|ApplyPointDamage otherActor (* (Variables|Default|GetDamage) (Default|GetDamageMultiplier (Variables|Default|Getattack))) (Math|Vector|MakeVector 0.0 0.0 0.0) (Collision|MakeHitResult false false 0.0 0.0 "0, 0, 0" "0, 0, 0" "0,0,1" "0,0,1" 0 otherActor component "None" "None" 0 0 0 "0, 0, 0" "0, 0, 0") (Pawn|GetController _aspawn) _aspawn "/Script/Engine.DamageType")))

(fn SpawnClaw
  (bind _asshiflix_character (Utilities|Casting|CastToShiflixCharacter (Components|GetOwner)))
  (bind _returnvalue (Game|SpawnActorfromClass (Variables|Default|GetarmType) (CallFunction|GetHitboxSpawn (Variables|Default|Getoffset)) "AlwaysSpawn" "MultiplyWithRoot" 0 3e+01 _asshiflix_character))
  (Transformation|AttachActorToActor _returnvalue (Components|GetOwner) "None" "KeepWorld" "KeepWorld" "KeepRelative" true)
  (Variables|/Script/Engine.Actor|SetTags _returnvalue (Utilities|Array|MakeArray "Player"))
  ;[1 1 1] Check overlaps on spawn
  (Collision|BindEventtoOnComponentBeginOverlap (Variables|/Game/Damage/BP_AttackArm.BP_AttackArm_C|GetHitBox _returnvalue) (EventDispatchers|CreateEvent :!event Custom|Overlap))
  (return _returnvalue))

(fn ShouldHit
  (params (actor :type Actor%20Object%20Reference%20%28by%20ref%29))
  (bind _output_get (LocalVariables|SetshouldHitTemp (and (== (Utilities|Array|FindItem (Variables|Default|GetattackedActors) actor) -1) (!= actor (Components|GetOwner)))))
  (if _output_get
    (Utilities|Array|Add (Variables|Default|GetattackedActors) actor))
  (return (LocalVariables|GetshouldHitTemp)))