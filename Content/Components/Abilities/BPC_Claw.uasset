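; Claw ability component that gives a ShiflixCharacter a melee slash attack.
; On BeginPlay it spawns a persistent BP_Slash actor in front of the owner, attaches it, tags it as Player and binds to its hitbox's begin-overlap.
; Use triggers the slash's Attack.
; Overlaps apply point damage credited to the owning pawn's controller, skipping actors that share the owner's instigator.
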(event Custom|Overlap
  (params (OverlappedComponent :type Primitive%20Component%20Object%20Reference) (OtherActor :type Actor%20Object%20Reference) (OtherComp :type Primitive%20Component%20Object%20Reference) (OtherBodyIndex :type Integer) (bFromSweep :type Boolean) (SweepResult :type Hit%20Result%20Structure%20%28by%20ref%29))
  (CallFunction|ApplyDamage (Variables|Default|GetDamage) OtherActor))

(event EventBeginPlay
  (bind _returnvalue (CallFunction|SpawnClaw))
  (Variables|Default|SetClaw _returnvalue))

(event EventUse
  (Default|Attack (Variables|Default|GetClaw)))

(fn GetHitboxSpawn
  (params (offset :type Float%20%28double-precision%29))
  (bind _returnvalue (Components|GetOwner))
  (bind _returnvalue_2 (Transformation|GetActorForwardVector _returnvalue))
  (return (Math|Transform|MakeTransform (+ (Transformation|GetActorLocation _returnvalue) (* _returnvalue_2 offset)) (Math|Conversions|RotationFromXVector _returnvalue_2) "1.000000,1.000000,1.000000")))

(fn ApplyDamage
  (params (damage :type Float%20%28double-precision%29) (otherActor :type Actor%20Object%20Reference))
  (bind _aspawn (Utilities|Casting|CastToPawn (Components|GetOwner)))
  (if (!= (Variables|/Script/Engine.Actor|GetInstigator _aspawn) (Variables|/Script/Engine.Actor|GetInstigator otherActor))
    (Game|Damage|ApplyPointDamage otherActor (Variables|Default|GetDamage) (Math|Vector|MakeVector 0.0 0.0 0.0) (Collision|MakeHitResult false false 0.0 0.0 "0, 0, 0" "0, 0, 0" "0,0,1" "0,0,1" 0 0 0 "None" "None" 0 0 0 "0, 0, 0" "0, 0, 0") (Pawn|GetController _aspawn) _aspawn "/Script/Engine.DamageType")))

(fn SpawnClaw
  (bind _asshiflix_character (Utilities|Casting|CastToShiflixCharacter (Components|GetOwner)))
  (bind _returnvalue (Game|SpawnActorfromClass "/Game/Damage/BP_Slash.BP_Slash_C" (CallFunction|GetHitboxSpawn 1e+02) "AlwaysSpawn" "MultiplyWithRoot" 0 3e+01 _asshiflix_character))
  (Transformation|AttachActorToActor _returnvalue (Components|GetOwner) "None" "KeepWorld" "KeepWorld" "KeepRelative" true)
  (Variables|/Script/Engine.Actor|SetTags _returnvalue (Utilities|Array|MakeArray "Player"))
  ;[1 1 1] Check overlaps on spawn
  (Collision|BindEventtoOnComponentBeginOverlap (Variables|/Game/Damage/BP_Slash.BP_Slash_C|GetHitBox _returnvalue) (EventDispatchers|CreateEvent :!event Custom|Overlap))
  (return _returnvalue))