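; Damageable body-part component that detects hits from tagged actors, accumulates damage and can drop itself as a limb pickup.
; On BeginPlay it binds overlap events on its child box and capsule colliders, counting overlaps so damage start and end fire only on the first and last.
; Damage only adds to a total.
; Drop spawns BP_LimbPickup with its slot and ability, then destroys itself and its children.
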(event Custom|Overlap
  (params (OverlappedComponent :type Primitive%20Component%20Object%20Reference) (OtherActor :type Actor%20Object%20Reference) (OtherComp :type Primitive%20Component%20Object%20Reference) (OtherBodyIndex :type Integer) (bFromSweep :type Boolean) (SweepResult :type Hit%20Result%20Structure%20%28by%20ref%29))
  (if (Actor|ActorHasTag OtherActor (Variables|Default|GetTag))
    (if (CallFunction|IsHit)
      _
      (else
        (Default|CallStartDamage)))
    (Math|Integer|IncrementInt (Variables|Default|GetnrHits))))

(event Custom|EndOverlap
  (params (OverlappedComponent :type Primitive%20Component%20Object%20Reference) (OtherActor :type Actor%20Object%20Reference) (OtherComp :type Primitive%20Component%20Object%20Reference) (OtherBodyIndex :type Integer))
  (if (Actor|ActorHasTag OtherActor (Variables|Default|GetTag))
    (Math|Integer|DecrementInt (Variables|Default|GetnrHits)
      (:%20%20
        (if (not (CallFunction|IsHit))
          (Default|CallEndDamage))))))

(event EventBeginPlay
  (CallFunction|ApplyDelegates))

(event EventTick
  (params (DeltaSeconds :type Float%20%28single-precision%29)))

(fn ApplyDelegates
  (Utilities|FlowControl|Sequence
    (:then_0
      ;[1 1 1] Collect collisions
      (for _array_element (Components|GetChildrenComponents true)
        (bind _asbox_collision (Utilities|Casting|CastToBoxComponent _array_element)
          (:then
            (Utilities|Array|Add (LocalVariables|GetcollisionBoxes) _asbox_collision))
          (:CastFailed
            (bind _ascapsule_collision (Utilities|Casting|CastToCapsuleComponent _array_element))
            (Utilities|Array|Add (LocalVariables|GetcollisionCapsules) _ascapsule_collision)))))
    (:then_1
      (for _array_element_2 (LocalVariables|GetcollisionCapsules)
        (Collision|BindEventtoOnComponentBeginOverlap _array_element_2 (EventDispatchers|CreateEvent :!event Custom|Overlap))
        (Collision|BindEventtoOnComponentEndOverlap _array_element_2 (EventDispatchers|CreateEvent :!event Custom|EndOverlap))))
    (:then_2
      (for _array_element_3 (LocalVariables|GetcollisionBoxes)
        (Collision|BindEventtoOnComponentBeginOverlap _array_element_3 (EventDispatchers|CreateEvent :!event Custom|Overlap))
        (Collision|BindEventtoOnComponentEndOverlap _array_element_3 (EventDispatchers|CreateEvent :!event Custom|EndOverlap))))))

(fn Drop
  (if (CallFunction|CanSpawnLimb)
    (Utilities|FlowControl|Sequence
      (:then_0
        ;[1 1 1] Spawn pickup
        (bind _aspawn (Utilities|Casting|CastToPawn (Components|GetOwner)))
        (Game|SpawnActorfromClass "/Game/Interactibles/BP_LimbPickup.BP_LimbPickup_C" (Transformation|GetWorldTransform) "AdjustIfPossibleButAlwaysSpawn" "MultiplyWithRoot" 0 (Variables|Default|GetbodyPartSlot) (Variables|Default|GetabilityType) _aspawn))
      (:then_1
        ;[1 1 1] Remove limb
        (for _array_element (Components|GetChildrenComponents true)
          (Components|DestroyComponent _array_element))
        (Components|DestroyComponent)))))

(fn CanSpawnLimb
  ;[1 1 1] Check if valid input
  (return (and (Utilities|IsValidClass (Variables|Default|GetabilityType)) (Utilities|Enum|NotEqual(Enum) (Variables|Default|GetbodyPartSlot) "none"))))

(fn IsHit
  (return (> (Variables|Default|GetnrHits) 0)))

(fn Damage
  (params (Damage :type Float%20%28double-precision%29))
  (Variables|Default|SetaccumDamage (+ Damage (Variables|Default|GetaccumDamage))))

(fn GetTotalDamage
  (return (Variables|Default|GetaccumDamage)))