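; Health component that tracks a clamped health value, fires a depleted event at zero and optionally regenerates over time.
; Damage lowers health, halts regeneration and restarts a delay timer, and Tick replenishes at the regen rate while regeneration is active.
; Replenish reuses Damage with a negated amount, restoring the regen flag afterward but also restarting the timer.
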(event EventBeginPlay
  (CallFunction|Reset))

(event EventTick
  (params (DeltaSeconds :type Float%20%28single-precision%29))
  (if (and (Variables|Default|GetautoRegen) (Variables|Default|GetisRegening))
    (CallFunction|Replenish (* DeltaSeconds (Variables|Default|GetRegenRate)))))

(fn Damage
  (params (damage :type Float%20%28double-precision%29))
  (Utilities|FlowControl|Sequence
    (:then_0
      (bind _output_get (Variables|Default|Sethealth (Math|Float|Clamp(Float) (- (Variables|Default|Gethealth) damage) 0.0 (Variables|Default|GetmaxHealth))))
      (if (<= _output_get 0.0)
        (Default|CallHealthDepleted)))
    (:then_1
      (Variables|Default|SetIsDamaged true)
      (Variables|Default|SetisRegening false)
      (Utilities|Time|InvalidateTimerHandle (Variables|Default|GetregenTimerHandle))
      (bind _returnvalue (Utilities|Time|SetTimerbyEvent (EventDispatchers|CreateEvent :!event SetRegen) (Variables|Default|GetRegenDelay)))
      (Variables|Default|SetregenTimerHandle _returnvalue))))

(fn Replenish
  (params (health :type Float%20%28double-precision%29))
  (LocalVariables|SetisRegeningtemp (Variables|Default|GetisRegening))
  (CallFunction|Damage (* health -1.0))
  (Variables|Default|SetIsDamaged false)
  (Variables|Default|SetisRegening (LocalVariables|GetisRegeningtemp)))

(fn Reset
  (Variables|Default|Sethealth (Variables|Default|GetmaxHealth)))

(fn GetHealthRatio
  (return (/ (Variables|Default|Gethealth) (Variables|Default|GetmaxHealth))))

(fn SetRegen
  (Variables|Default|SetisRegening true))