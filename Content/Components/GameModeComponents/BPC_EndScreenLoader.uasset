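; Game mode component that shows the death screen when the player character dies.
; It binds LoadEnd to the player's DeathHandler delegate on BeginPlay and again on the first Tick.
; LoadEnd fills BPW_DeathScreen with survival time and kill count from the owner's BPC_Stats and adds it to the viewport.
; It then pauses the game, shows the cursor, focuses input on the widget and calls SwapControls on the player.
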(event Custom|LoadEnd
  (params (character :type Shiflix%20Character%20Object%20Reference))
  (bind _returnvalue (Components|GetOwner))
  (bind _returnvalue_2 (Game|GetPlayerController 0))
  (bind _returnvalue_3 (Actor|GetComponentbyClass _returnvalue "/Game/Components/GameModeComponents/BPC_Stats.BPC_Stats_C"))
  (bind _returnvalue_4 (Game|ConstructObjectfromClass "/Game/HUD/BPW_DeathScreen.BPW_DeathScreen_C"))
  (Variables|/Game/HUD/BPW_DeathScreen.BPW_DeathScreen_C|SetsurvivalTime _returnvalue_4 (Variables|/Game/Components/GameModeComponents/BPC_Stats.BPC_Stats_C|GetsurvivalTime _returnvalue_3))
  (Variables|/Game/HUD/BPW_DeathScreen.BPW_DeathScreen_C|SetnrKills _returnvalue_4 (Variables|/Game/Components/GameModeComponents/BPC_Stats.BPC_Stats_C|GetnrKills _returnvalue_3))
  (UserInterface|Viewport|AddtoViewport _returnvalue_4 0)
  (Game|SetGamePaused true)
  (Variables|/Script/Engine.PlayerController|SetbShowMouseCursor _returnvalue_2 true)
  (Input|SetInputModeGameandUI _returnvalue_2 _returnvalue_4 "DoNotLock" true false)
  (bind _asbp_player_character (Utilities|Casting|CastToBP_PlayerCharacter (Game|GetPlayerCharacter 0)))
  (Default|SwapControls _asbp_player_character))

(event EventBeginPlay
  (bind _asbp_player_character (Utilities|Casting|CastToBP_PlayerCharacter (Game|GetPlayerCharacter 0)))
  (EventDispatchers|BindEventtoDeathDelegate (Variables|/Script/ProjectElementP1.ShiflixCharacter|GetDeathHandler _asbp_player_character) (delegate Custom|LoadEnd)))

(event EventTick
  (params (DeltaSeconds :type Float%20%28single-precision%29))
  (if (not (Variables|Default|Getloaded))
    (Variables|Default|Setloaded true)
    (bind _asbp_player_character (Utilities|Casting|CastToBP_PlayerCharacter (Game|GetPlayerCharacter 0)))
    (EventDispatchers|BindEventtoDeathDelegate (Variables|/Script/ProjectElementP1.ShiflixCharacter|GetDeathHandler _asbp_player_character) (delegate Custom|LoadEnd))))