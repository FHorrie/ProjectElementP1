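; BPC_Spawner is a game mode component that runs escalating waves of Imp enemies.
; On BeginPlay it gathers the BP_Spawner actors, then starts a wave, growing the enemy count by half each time.
; A looping timer spawns Imps at random points until the quota is met, binding each one's death delegate.
; Deaths update wave counters; when no spawned enemies remain, it advances the wave and starts a grace timer, notifying through wave events.
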(event EventBeginPlay
  (bind _outactors (Actor|GetAllActorsOfClass "/Game/Level/BP_Spawner.BP_Spawner_C"))
  (bind _output_get (Variables|Spawning|SetSpawnPoints _outactors))
  (Variables|Spawning|SetSpawnPointsAmount (Utilities|Array|Length _output_get))
  (Utilities|FlowControl|Delay 0.1)
  (CallFunction|SpawnWave))

(fn HandleDeadEnemy
  (params (Enemy :type Shiflix%20Character%20Object%20Reference))
  (Math|Integer|DecrementInt (Variables|WaveSystem|GetWaveEnemiesRemaining)
    (:%20%20
      (bind _result (Math|Integer|DecrementInt (Variables|WaveSystem|GetEnemySpawnedCount))
        (:%20%20
          (Default|CallWaveStateChanged)
          (if (== _result 0)
            (Math|Integer|IncrementInt (Variables|WaveSystem|GetCurrentWave)
              (:%20%20
                (Utilities|Time|SetTimerbyEvent (EventDispatchers|CreateEvent :!event SpawnWave) (Variables|Default|GetGraceTime))
                (Default|CallGraceStarting)))))))))

(fn HandleSpawnEnemy
  (if (== (Variables|WaveSystem|GetEnemiesSpawnedThisWave) (Variables|WaveSystem|GetWaveEnemies))
    (Utilities|Time|InvalidateTimerHandle (Variables|Spawning|GetSpawnerHandle))
    (else
      (CallFunction|SpawnEnemy))))

(fn SpawnEnemy
  ;[0.1094 0.1094 0.1094] Spawning logics
  (bind _returnvalue (Game|SpawnActorfromClass "/Game/Player/BP_Imp.BP_Imp_C" (Math|Transform|MakeTransform (Transformation|GetActorLocation (.OutItem (Utilities|Array|Random (Variables|Spawning|GetSpawnPoints)))) "0, 0, 0" "1.000000,1.000000,1.000000") "AdjustIfPossibleButAlwaysSpawn" "MultiplyWithRoot" 0 0))
  (EventDispatchers|BindEventtoDeathDelegate (Variables|/Script/ProjectElementP1.ShiflixCharacter|GetDeathHandler _returnvalue) (EventDispatchers|CreateEvent :!event HandleDeadEnemy))
  (Math|Integer|IncrementInt (Variables|WaveSystem|GetEnemySpawnedCount)
    (:%20%20
      (Math|Integer|IncrementInt (Variables|WaveSystem|GetEnemiesSpawnedThisWave)))))

(fn SpawnWave
  (Variables|WaveSystem|SetEnemiesSpawnedThisWave 0)
  (bind _output_get (Variables|WaveSystem|SetWaveEnemies (+ (Variables|WaveSystem|GetWaveEnemies) (/ (Variables|WaveSystem|GetWaveEnemies) 2))))
  (Variables|WaveSystem|SetWaveEnemiesRemaining _output_get)
  (Default|CallWaveStateChanged)
  (Default|CallWaveStarting)
  (bind _returnvalue (Utilities|Time|SetTimerbyEvent (EventDispatchers|CreateEvent :!event HandleSpawnEnemy) 1.0 true))
  (Variables|Spawning|SetSpawnerHandle _returnvalue))