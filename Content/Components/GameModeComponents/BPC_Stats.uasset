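; Game mode component that tracks run statistics: survival time and kill count.
; It binds to wave-start, grace-start and enemy-death events of the BPC_Spawner on its owner, both at BeginPlay and again on the first Tick.
; Subsequent ticks accumulate survival time unless paused, with functions to pause, unpause and increment kills.
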(event EventBeginPlay
  (bind _returnvalue (Components|GetOwner))
  (bind _returnvalue_2 (Actor|GetComponentbyClass _returnvalue "/Game/Components/GameModeComponents/BPC_Spawner.BPC_Spawner_C"))
  ;[1 1 1] Setup events
  (EventDispatchers|BindEventtoWaveStarting _returnvalue_2 (EventDispatchers|CreateEvent :!event Unpause))
  (EventDispatchers|BindEventtoGraceStarting _returnvalue_2 (EventDispatchers|CreateEvent :!event Pause))
  (EventDispatchers|BindEventtoEnemyDied _returnvalue_2 (EventDispatchers|CreateEvent :!event AddKill)))

(event EventTick
  (params (DeltaSeconds :type Float%20%28single-precision%29))
  (bind _returnvalue (Components|GetOwner))
  (bind _returnvalue_2 (Actor|GetComponentbyClass _returnvalue "/Game/Components/GameModeComponents/BPC_Spawner.BPC_Spawner_C"))
  (if (Variables|Default|Getloaded)
    (CallFunction|AddTime DeltaSeconds)
    (else
      (Variables|Default|Setloaded true)
      ;[1 1 1] Setup events
      (EventDispatchers|BindEventtoWaveStarting _returnvalue_2 (EventDispatchers|CreateEvent :!event Unpause))
      (EventDispatchers|BindEventtoGraceStarting _returnvalue_2 (EventDispatchers|CreateEvent :!event Pause))
      (EventDispatchers|BindEventtoEnemyDied _returnvalue_2 (EventDispatchers|CreateEvent :!event AddKill)))))

(fn AddTime
  (params (deltaTime :type Float%20%28double-precision%29))
  (if (not (Variables|Default|GetisPaused))
    (Variables|Default|SetsurvivalTime (+ deltaTime (Variables|Default|GetsurvivalTime)))))

(fn Pause
  (Variables|Default|SetisPaused true))

(fn Unpause
  (Variables|Default|SetisPaused false))

(fn AddKill
  (Math|Integer|IncrementInt (Variables|Default|GetnrKills)))