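; BPC_ShopOwner is a game mode component that opens and closes the base station shop in step with enemy wave phases.
; On BeginPlay it caches the owner's BPC_Spawner and finds the BP_BaseStation in the level.
; It binds to the spawner's grace-starting and wave-starting events, calling OpenStation during grace periods and CloseStation when a wave begins.
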(event Custom|OpenShop
  (Default|OpenStation (Variables|Default|GetbaseStation)))

(event Custom|CloseShop
  (Default|CloseStation (Variables|Default|GetbaseStation)))

(event EventBeginPlay
  (Utilities|FlowControl|Sequence
    (:then_0
      (Variables|Default|SetwaveComp (Actor|GetComponentbyClass (Components|GetOwner) "/Game/Components/GameModeComponents/BPC_Spawner.BPC_Spawner_C"))
      (bind _returnvalue (Actor|GetActorOfClass "/Game/Interactibles/BP_BaseStation.BP_BaseStation_C"))
      (Variables|Default|SetbaseStation _returnvalue))
    (:then_1
      (EventDispatchers|BindEventtoGraceStarting (Variables|Default|GetwaveComp) (delegate Custom|OpenShop))
      (EventDispatchers|BindEventtoWaveStarting (Variables|Default|GetwaveComp) (delegate Custom|CloseShop)))))