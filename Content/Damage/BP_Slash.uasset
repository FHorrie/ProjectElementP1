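; BP_Slash is a combo bear-claw melee attack that swaps a placeholder for the claw mesh during each swing.
; Attack starts a swing; Tick plays the AllowHit timeline, moving the claw along the current spline path, oriented by its tangent.
; Timeline events toggle hitbox overlaps; finishing hides the claw, advances the combo and re-allows attacks after a short delay.
; A retriggerable delay resets the combo, while Interrupt resets it and stops the timeline.
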(event Custom|Interrupt
  (CallFunction|Reset)
  (bind _lerpvalue (Timeline|AllowHit Stop)
    (:Update
      (Transformation|SetRelativeLocationAndRotation (Variables|Default|GetClaw) (.location (CallFunction|GetClawTransform (Utilities|Array|Get(acopy) (Variables|Default|Getattacks) (Variables|Default|GetcurrentCombo)) _lerpvalue)) (.rotation (CallFunction|GetClawTransform (Utilities|Array|Get(acopy) (Variables|Default|Getattacks) (Variables|Default|GetcurrentCombo)) _lerpvalue)) false true))
    (:Finished
      (CallFunction|Hide)
      (Utilities|FlowControl|Delay 0.5)
      (Variables|Default|SetallowAttack true)
      (Timeline|AllowHit SetNewTime))
    (:Toggle
      (CallFunction|ToggleHit))))

(event Custom|Attack
  (if (Variables|Default|GetallowAttack)
    (CallFunction|Unhide)
    (Variables|Default|SetallowAttack false)))

(event EventBeginPlay
  ;[1 1 1] GetAttackPaths
  (Variables|Default|Setattacks (Utilities|Array|MakeArray (Variables|Default|GetAttackPath) (Variables|Default|GetAttackPath1))))

(event EventTick
  (params (DeltaSeconds :type Float%20%28single-precision%29))
  (if (Variables|Default|GetisAttacking)
    (Utilities|FlowControl|Sequence
      (:then_0
        (bind _lerpvalue (Timeline|AllowHit Play)
          (:Update
            (Transformation|SetRelativeLocationAndRotation (Variables|Default|GetClaw) (.location (CallFunction|GetClawTransform (Utilities|Array|Get(acopy) (Variables|Default|Getattacks) (Variables|Default|GetcurrentCombo)) _lerpvalue)) (.rotation (CallFunction|GetClawTransform (Utilities|Array|Get(acopy) (Variables|Default|Getattacks) (Variables|Default|GetcurrentCombo)) _lerpvalue)) false true))
          (:Finished
            (CallFunction|Hide)
            (Utilities|FlowControl|Delay 0.5)
            (Variables|Default|SetallowAttack true)
            (Timeline|AllowHit SetNewTime))
          (:Toggle
            (CallFunction|ToggleHit))))
      (:then_1
        (Utilities|FlowControl|RetriggerableDelay (Variables|Default|GetresetTime))
        (CallFunction|Reset)))))

(fn ConstructionScript)

(fn ToggleHit
  (bind _hitbox (Variables|Default|GetHitBox))
  (Variables|/Script/Engine.PrimitiveComponent|SetbGenerateOverlapEvents _hitbox (not (Variables|/Script/Engine.PrimitiveComponent|GetbGenerateOverlapEvents _hitbox))))

(fn Hide
  (Variables|/Script/Engine.PrimitiveComponent|SetbGenerateOverlapEvents (Variables|Default|GetHitBox) false)
  (Rendering|SetVisibility (Variables|Default|GetMesh_BearClaw1) false true)
  (bind _result (Math|Integer|IncrementInt (Variables|Default|GetcurrentCombo))
    (:%20%20
      (Variables|Default|SetcurrentCombo (Math|Integer|%(Integer) _result (Utilities|Array|Length (Variables|Default|Getattacks))))
      (Rendering|SetVisibility (Variables|Default|GetPlaceholder) true true)
      (Variables|Default|SetisAttacking false))))

(fn Unhide
  (Rendering|SetVisibility (Variables|Default|GetMesh_BearClaw1) true true)
  (Variables|Default|SetisAttacking true)
  (Rendering|SetVisibility (Variables|Default|GetPlaceholder) false true))

(fn GetClawTransform
  (params (spline :type Spline%20Component%20Object%20Reference) (alpha :type Float%20%28double-precision%29))
  (bind _duration (Variables|/Script/Engine.SplineComponent|GetDuration spline))
  (bind _returnvalue (* _duration alpha))
  (return (Spline|GetLocationatTime spline _returnvalue "Local" false) (Math|Conversions|RotationFromXVector (Class|SplineComponent|GetTangentatTime spline _returnvalue "Local" false))))

(fn Reset
  (Variables|Default|SetcurrentCombo 0)
  (Variables|Default|SetisAttacking false))