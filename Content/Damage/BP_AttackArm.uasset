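; Melee attack arm that plays combo strikes by moving an arm along its spline components, one spline per strike.
; Attack swaps the placeholder for the arm, then Tick drives it along the spline and toggles hitbox overlaps at normalized ToggleEvents times.
; Each finished strike hides the arm, advances the combo and re-allows attacking after that strike's delay.
; A retriggerable delay resets the combo after inactivity, Interrupt resets immediately, and BeginPlay reports setup errors.
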(event Custom|Interrupt
  (CallFunction|Hide)
  (CallFunction|Reset))

(event Custom|Attack
  (if (Variables|Default|GetallowAttack)
    (CallFunction|Unhide)
    (Variables|Default|SetallowAttack false)))

(event EventBeginPlay
  (bind _toggleevents (Variables|Default|GettoggleEvents))
  (bind _returnvalue (Utilities|Array|IsEmpty _toggleevents))
  (Variables|Default|Setattacks (Actor|GetComponentsByClass "/Script/Engine.SplineComponent"))
  (CallFunction|Hide)
  (CallFunction|Reset)
  ;[1 1 1] debug checking
  (Utilities|FlowControl|Sequence
    (:then_0
      ;;[1 1 1] SPlines check
      (Development|PrintString (CallFunction|GetErrorMessage "No splines found in attack arm: ") (Utilities|Array|IsEmpty (Variables|Default|Getattacks)) (Utilities|Array|IsEmpty (Variables|Default|Getattacks))))
    (:then_1
      ;;[1 1 1] Toggle events check
      (Development|PrintString (CallFunction|GetErrorMessage "No toggle events found in attack arm: ") _returnvalue _returnvalue))
    (:then_2
      ;;[1 1 1] Toggle events check
      (Development|PrintString (CallFunction|GetErrorMessage "The attack delay count is not the same as the nr of attack strikes: ") (!= (Utilities|Array|Length (Variables|Default|GetattackDelay)) (Utilities|Array|Length (Variables|Default|Getattacks))) (!= (Utilities|Array|Length (Variables|Default|GetattackDelay)) (Utilities|Array|Length (Variables|Default|Getattacks)))))))

(event EventTick
  (params (DeltaSeconds :type Float%20%28single-precision%29))
  (bind _attacks (Variables|Default|Getattacks))
  (bind _currentcombo (Variables|Default|GetcurrentCombo))
  (bind _output (Utilities|Array|Get(acopy) _attacks _currentcombo))
  (if (Variables|Default|GetisAttacking)
    (Utilities|FlowControl|Sequence
      (:then_0
        (bind _output_get (Variables|Default|Settimer (+ (Variables|Default|Gettimer) DeltaSeconds)))
        (for (_array_element _array_index) (Variables|Default|GettoggledEvents)
          (if (<= _array_element (/ _output_get (Variables|/Script/Engine.SplineComponent|GetDuration _output)))
            (CallFunction|ToggleHit)
            ;[1 1 1] Set to a value that will never be hit
            (Utilities|Array|SetArrayElem (Variables|Default|GettoggledEvents) _array_index 2.0)))
        ;[1 1 1] Bring arm alongside spline
        (Transformation|SetRelativeLocationAndRotation (Variables|Default|Getarm) (.location (CallFunction|GetClawTransform _output (/ _output_get (Variables|/Script/Engine.SplineComponent|GetDuration _output)))) (.rotation (CallFunction|GetClawTransform _output (/ _output_get (Variables|/Script/Engine.SplineComponent|GetDuration _output)))) false true)
        (if (>= (/ _output_get (Variables|/Script/Engine.SplineComponent|GetDuration _output)) 1.0)
          ;[1 1 1] Next attack setup
          (bind _delay (CallFunction|GetAttackDelay))
          (CallFunction|Hide)
          (Utilities|FlowControl|Delay _delay)
          (Variables|Default|SetallowAttack true)))
      (:then_1
        (Utilities|FlowControl|RetriggerableDelay (Variables|Default|GetresetTime))
        (CallFunction|Reset)))))

(fn ConstructionScript)

(fn ToggleHit
  (bind _hitbox (Variables|Default|GetHitBox))
  (Variables|/Script/Engine.PrimitiveComponent|SetbGenerateOverlapEvents _hitbox (not (Variables|/Script/Engine.PrimitiveComponent|GetbGenerateOverlapEvents _hitbox))))

(fn Hide
  (Variables|/Script/Engine.PrimitiveComponent|SetbGenerateOverlapEvents (Variables|Default|GetHitBox) false)
  (Rendering|SetVisibility (Variables|Default|Getarm) false true)
  (bind _result (Math|Integer|IncrementInt (Variables|Default|GetcurrentCombo))
    (:%20%20
      (Variables|Default|SetcurrentCombo (Math|Integer|%(Integer) _result (Utilities|Array|Length (Variables|Default|Getattacks))))
      (Rendering|SetVisibility (Variables|Default|GetPlaceholder) true true)
      (Variables|Default|SetisAttacking false)
      (Variables|Default|SettoggledEvents (Variables|Default|GettoggleEvents))
      (Variables|Default|Settimer 0.0))))

(fn Unhide
  (Rendering|SetVisibility (Variables|Default|Getarm) true true)
  (Variables|Default|SetisAttacking true)
  (Rendering|SetVisibility (Variables|Default|GetPlaceholder) false true))

(fn GetClawTransform
  (params (spline :type Spline%20Component%20Object%20Reference) (alpha :type Float%20%28double-precision%29))
  (bind _duration (Variables|/Script/Engine.SplineComponent|GetDuration spline))
  (bind _returnvalue (* _duration alpha))
  (return (Spline|GetLocationatTime spline _returnvalue "Local" false) (Math|Conversions|RotationFromXVector (Class|SplineComponent|GetTangentatTime spline _returnvalue "Local" false))))

(fn Reset
  (Variables|Default|SetcurrentCombo 0)
  (Variables|Default|SetisAttacking false)
  (Variables|Default|SettoggledEvents (Variables|Default|GettoggleEvents))
  (Variables|Default|Settimer 0.0))

(fn GetAttackDelay
  (return (Utilities|Array|Get(acopy) (Variables|Default|GetattackDelay) (Variables|Default|GetcurrentCombo))))

(fn GetErrorMessage
  (params (Error :type String))
  (return (Utilities|String|Append Error ": " (Utilities|GetDisplayName self))))