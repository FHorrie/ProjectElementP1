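; Sword damage actor that adjusts its mesh pose to suit the current combo attack, extending a parent that provides Hide, Reset and attack timing.
; SetSwordPos sets a hard-coded relative rotation and location per combo step on BeginPlay, Hide and Reset.
; Tick inverts the blade once past the halfway point of the first two attacks, using a DoOnce that resets whenever that condition is false.
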(event EventBeginPlay
  (|CallParentFunction)
  (CallFunction|SetSwordPos))

(event Collision|EventActorBeginOverlap
  (params (OtherActor :type Actor%20Object%20Reference)))

(event EventTick
  (params (DeltaSeconds :type Float%20%28single-precision%29))
  (bind _staticmesh1 (Variables|Default|GetStaticMesh1))
  (|CallParentFunction DeltaSeconds)
  ;[1 1 1] Ugly way of inverting sword
  (if (and (or (== (Variables|Default|GetcurrentCombo) 0) (== (Variables|Default|GetcurrentCombo) 1)) (> (/ (Variables|Default|Gettimer) (Variables|/Script/Engine.SplineComponent|GetDuration (Utilities|Array|Get(acopy) (Variables|Default|Getattacks) (Variables|Default|GetcurrentCombo)))) 0.5))
    (Utilities|FlowControl|DoOnce false :!label _label
      (:Completed
        (Transformation|SetRelativeRotation _staticmesh1 (Math|Rotator|MakeRotator 0.0 -9e+01 -9e+01) false false)
        (Transformation|SetRelativeLocation _staticmesh1 "40.000000,0.000000,0.000000" false true)))
    (else
      (goto _label Reset))))

(fn ConstructionScript
  (|CallParentFunction))

(fn Hide
  (|CallParentFunction)
  (CallFunction|SetSwordPos))

(fn Reset
  (|CallParentFunction)
  (CallFunction|SetSwordPos))

(fn SetSwordPos
  (bind _staticmesh1 (Variables|Default|GetStaticMesh1))
  (bind _staticmesh1_2 (Variables|Default|GetStaticMesh1))
  (bind _staticmesh1_3 (Variables|Default|GetStaticMesh1))
  (Utilities|FlowControl|Sequence
    (:then_0
      (if (or (== (Variables|Default|GetcurrentCombo) 0) (== (Variables|Default|GetcurrentCombo) 1))
        (Transformation|SetRelativeRotation _staticmesh1_3 (Math|Rotator|MakeRotator 2.7e+02 2.7e+02 1.8e+02) false false)
        (Transformation|SetRelativeLocation _staticmesh1_3 "-40.000000,0.000000,0.000000" false true)))
    (:then_1
      (if (== (Variables|Default|GetcurrentCombo) 2)
        (Transformation|SetRelativeRotation _staticmesh1_2 (Math|Rotator|MakeRotator 0.0 0.0 1.8e+02) false false)
        (Transformation|SetRelativeLocation _staticmesh1_2 "0.000000,-40.000000,0.000000" false true)))
    (:then_2
      (if (== (Variables|Default|GetcurrentCombo) 3)
        (Transformation|SetRelativeRotation _staticmesh1 (Math|Rotator|MakeRotator 89.999999 0.0 0.0) false false)
        (Transformation|SetRelativeLocation _staticmesh1 "0.000000,0.000000,-40.000000" false true)))))