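; BP_Imp is an AI-driven Imp with a health component and two damageable arms.
; Point damage reduces health and sets a blackboard hit key unless IsDamaged is set, then also damages the last arm that signalled StartDamage.
; Only the right arm's EndDamage is bound, clearing IsDamaged, which nothing here sets true.
; Health depletion triggers the DeathHandler and destroys the actor.
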(event HealthDepleted(BPC_Health)
  (Class|DeathComponent|Die (Variables|Default|GetDeathHandler))
  (Actor|DestroyActor))

(event Custom|StartDamage_Event
  ;[1 1 1] Would need damage
  (Variables|Default|SetDamagedPart (Variables|Default|GetRightArm)))

(event Custom|CustomEvent
  (Variables|Default|SetDamagedPart (Variables|Default|GetLeftArm)))

(event Custom|EndDamage_Event
  (Variables|Default|SetIsDamaged false))

(event EventBeginPlay
  (bind _rightarm (Variables|Default|GetRightArm))
  (EventDispatchers|AssignStartDamage _rightarm (delegate Custom|StartDamage_Event))
  (EventDispatchers|AssignEndDamage _rightarm (delegate Custom|EndDamage_Event))
  (EventDispatchers|BindEventtoStartDamage (Variables|Default|GetLeftArm) (delegate Custom|CustomEvent)))

(event Collision|EventActorBeginOverlap
  (params (OtherActor :type Actor%20Object%20Reference)))

(event EventTick
  (params (DeltaSeconds :type Float%20%28single-precision%29)))

(event Game|Damage|EventPointDamage
  (params (Damage :type Float%20%28single-precision%29) (DamageType :type Damage%20Type%20Object%20Reference) (HitLocation :type Vector :default "0, 0, 0") (HitNormal :type Vector :default "0, 0, 0") (HitComponent :type Primitive%20Component%20Object%20Reference) (BoneName :type Name :default "None") (ShotFromDirection :type Vector :default "0, 0, 0") (InstigatedBy :type Controller%20Object%20Reference) (DamageCauser :type Actor%20Object%20Reference) (HitInfo :type Hit%20Result%20Structure%20%28by%20ref%29))
  (bind _damagedpart (Variables|Default|GetDamagedPart))
  (CallFunction|Damage Damage)
  (Utilities|IsValid _damagedpart
    (:Is%20Valid
      (Default|Damage _damagedpart Damage))))

(fn ConstructionScript)

(fn Damage
  (params (Damage :type Float%20%28double-precision%29))
  (if (not (Variables|Default|GetIsDamaged))
    (AI|Components|Blackboard|SetValueasBool (AI|GetBlackboard 0) (Variables|Default|GetHitKey) true)
    (Default|Damage (Variables|Default|GetBPC_Health) Damage)))