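; HUD Blueprint that creates the wave counter and upgrade menu widgets, starting with the menu collapsed.
; ToggleUpgradeMenu uses UIState to swap widget visibility, cursor and input mode, then calls SwapControls on BP_PlayerCharacter.
; It leaves the game unpaused in both states.
; The player character's CloseEvent triggers CloseHud, which toggles the menu only when it is open.
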(event Custom|CloseHud
  (if (== (Variables|Default|GetUIState) 1)
    (CallFunction|ToggleUpgradeMenu)))

(event EventBeginPlay
  (Utilities|FlowControl|Sequence
    (:then_0
      (bind _returnvalue (Game|ConstructObjectfromClass "/Game/HUD/WBP_WaveCounter.WBP_WaveCounter_C"))
      (bind _output_get (Variables|Default|SetWaveCounterRef _returnvalue))
      (UserInterface|Viewport|AddtoViewport _output_get 0)
      (bind _returnvalue_2 (Game|ConstructObjectfromClass "/Game/HUD/WBP_UpgradeMenu.WBP_UpgradeMenu_C"))
      (bind _output_get_2 (Variables|Default|SetUpgradeMenuRef _returnvalue_2))
      (UserInterface|Viewport|AddtoViewport _output_get_2 0)
      (Widget|SetVisibility _output_get_2 "Collapsed"))
    (:then_1
      (bind _asbp_player_character (Utilities|Casting|CastToBP_PlayerCharacter (Game|Player|GetPlayerPawn 0)))
      (EventDispatchers|BindEventtoCloseEvent _asbp_player_character (delegate Custom|CloseHud)))))

(fn ConstructionScript)

(fn ToggleUpgradeMenu
  (bind _returnvalue (Game|GetPlayerController 0))
  (switch int (Variables|Default|GetUIState)
    (:0
      (Widget|SetVisibility (Variables|Default|GetWaveCounterRef) "Collapsed")
      (Widget|SetVisibility (Variables|Default|GetUpgradeMenuRef) "Visible")
      (Variables|Default|SetUIState 1)
      (Game|SetGamePaused false)
      (Variables|/Script/Engine.PlayerController|SetbShowMouseCursor _returnvalue true)
      (Input|SetInputModeGameandUI _returnvalue (Variables|Default|GetUpgradeMenuRef) "DoNotLock" true false))
    (:1
      (Widget|SetVisibility (Variables|Default|GetUpgradeMenuRef) "Collapsed")
      (Widget|SetVisibility (Variables|Default|GetWaveCounterRef) "Visible")
      (Variables|Default|SetUIState 0)
      (Game|SetGamePaused false)
      (Variables|/Script/Engine.PlayerController|SetbShowMouseCursor _returnvalue false)
      (Input|SetInputModeGameOnly _returnvalue false)))
  (bind _asbp_player_character (Utilities|Casting|CastToBP_PlayerCharacter (Game|Player|GetPlayerPawn 0)))
  (Default|SwapControls _asbp_player_character))